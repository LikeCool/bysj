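; BP_ConsoleCommandHandler exposes the game's console over HTTP through an embedded web server.
; BeginPlay starts the shared server instance on port 8080 and registers a /console handler for all methods on the game thread; EndPlay stops it.
; The handler executes the "command" POST variable as a console command without any validation, then replies with a fixed "test" response rather than the command's output.
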(event Custom|CustomEvent_0
  (params (Connection :type Connection%20Object%20Reference))
  (Development|ExecuteConsoleCommand (Class|Connection|GetPOSTVar Connection "command"))
  (Class|Connection|SendResponse Connection (Class|Response|ConstructResponseExt "test")))

(event EventBeginPlay
  (bind _returnvalue (Class|WebServer|GetorCreateWebServerInstance))
  (Class|WebServer|StartServer _returnvalue 8080 "www")
  (Class|WebServer|AddURIHandler _returnvalue "/console" (delegate Custom|CustomEvent_0) "VE_ALL" true))

(event EventEndPlay
  (params (EndPlayReason :type EEndPlayReason%20Enum :default "Destroyed"))
  (bind _returnvalue (Class|WebServer|GetorCreateWebServerInstance))
  (Class|WebServer|StopServer _returnvalue))

(fn ConstructionScript)